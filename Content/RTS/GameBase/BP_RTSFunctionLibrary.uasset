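; Blueprint function library that gives quick, typed access to the RTS game's core framework objects.
; Each function casts the game instance, game mode, player controller or player pawn (camera pawn) to its RTS class and returns it.
; Controller and pawn lookups always use player index 0, and a failed cast prints a red on-screen error instead of returning the object.
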(fn `FastGetRTSCameraPawn`
  (returns (`AsRTSCamera Pawn` :type "RTSCameraPawn Object Reference"))
  (bind _asrtscamera_pawn (cast `RTSCameraPawn` (`GameplayStatics.GetPlayerPawn` null))
    (:`then`
      (return _asrtscamera_pawn))
    (:`CastFailed`
      (`KismetSystemLibrary.PrintString` null "PlayerPawn Can't Cast To RTSCameraPawn" true true (struct :`R` 1.0 :`A` 1.0) 10.0))))

(fn `FastGetRTSGameInstance`
  (returns (`AsRTSGame Instance` :type "RTSGameInstance Object Reference"))
  (bind _asrtsgame_instance (cast `RTSGameInstance` (`GameplayStatics.GetGameInstance` null))
    (:`then`
      (return _asrtsgame_instance))
    (:`CastFailed`
      (`KismetSystemLibrary.PrintString` null "GameInstance Can't Cast To RTSGameInstance" true true (struct :`R` 1.0 :`A` 1.0) 10.0))))

(fn `FastGetRTSGameMode`
  (returns (`AsRTSGame Mode` :type "RTSGameMode Object Reference"))
  (bind _asrtsgame_mode (cast `RTSGameMode` (`GameplayStatics.GetGameMode` null))
    (:`then`
      (return _asrtsgame_mode))
    (:`CastFailed`
      (`KismetSystemLibrary.PrintString` null "GameMode Can't Cast To RTSGameMode" true true (struct :`R` 1.0 :`A` 1.0) 10.0))))

(fn `FastGetRTSPlayerController`
  (returns (`AsRTSPlayer Controller` :type "RTSPlayerController Object Reference"))
  (bind _asrtsplayer_controller (cast `RTSPlayerController` (`GameplayStatics.GetPlayerController` null))
    (:`then`
      (return _asrtsplayer_controller))
    (:`CastFailed`
      (`KismetSystemLibrary.PrintString` null "PlayerController Can't Cast To RTSPlayerController" true true (struct :`R` 1.0 :`A` 1.0) 10.0))))