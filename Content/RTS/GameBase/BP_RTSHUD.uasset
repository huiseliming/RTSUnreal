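; BP_RTSHUD is a Blueprint for the RTS HUD that highlights units as the selection hover moves over them.
; On BeginPlay it binds handlers to the RTS selection hovered and unhovered events, which show or hide the SelectedDecal on BP_RTSUnit actors.
; Despite the handlers' Selected and Deselected names, only hover drives the decal, as the selected and deselected bindings are disconnected and never run.
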(event `self.ReceiveBeginPlay`
  (add `self.OnRTSSelectionHovered` (delegate `OnRTSSelectionSelected_Event_0`))
  (add `self.OnRTSSelectionUnhovered` (delegate `OnRTSSelectionDeselected_Event_0`)))

(event `OnRTSSelectionSelected_Event_0` :!signature `self.OnRTSSelectionSelected`
  (params (Actor :type "Actor Object Reference"))
  (bind _asbp_rtsunit (cast `/Game/RTS/Unit/BP_RTSUnit` Actor))
  (`SceneComponent.SetVisibility` (`/Game/RTS/Unit/BP_RTSUnit.SelectedDecal` _asbp_rtsunit) true false))

(event `OnRTSSelectionDeselected_Event_0` :!signature `self.OnRTSSelectionDeselected`
  (params (Actor :type "Actor Object Reference"))
  (bind _asbp_rtsunit (cast `/Game/RTS/Unit/BP_RTSUnit` Actor))
  (`SceneComponent.SetVisibility` (`/Game/RTS/Unit/BP_RTSUnit.SelectedDecal` _asbp_rtsunit) false false))

(fn `UserConstructionScript`)