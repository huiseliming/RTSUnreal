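; Blueprint function library of shortcut getters for the core War3 framework objects: game instance, game mode, player controller and camera pawn.
; Each function fetches the engine object, using player index 0 for the controller and pawn, and casts it to its BP_War3 class.
; A failed cast prints a red on-screen error for ten seconds instead of returning the object.
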(fn `FastGetWar3CameraPawn`
  (returns (`AsBP War 3Camera Pawn` :type "/Game/War3/GameBase/BP_War3CameraPawn Object Reference"))
  (bind _asbp_war_3camera_pawn (cast `/Game/War3/GameBase/BP_War3CameraPawn` (`GameplayStatics.GetPlayerPawn` null))
    (:`then`
      (return _asbp_war_3camera_pawn))
    (:`CastFailed`
      (`KismetSystemLibrary.PrintString` null "PlayerPawn Can't Cast To BP_War3CameraPawn" true true (struct :`R` 1.0 :`A` 1.0) 10.0))))

(fn `FastGetWar3GameInstance`
  (returns (`AsBP War 3Game Instance` :type "/Game/War3/GameBase/BP_War3GameInstance Object Reference"))
  (bind _asbp_war_3game_instance (cast `/Game/War3/GameBase/BP_War3GameInstance` (`GameplayStatics.GetGameInstance` null))
    (:`then`
      (return _asbp_war_3game_instance))
    (:`CastFailed`
      (`KismetSystemLibrary.PrintString` null "GameInstance Can't Cast To BP_War3GameInstance" true true (struct :`R` 1.0 :`A` 1.0) 10.0))))

(fn `FastGetWarGameMode`
  (returns (`AsBP War 3Game Mode` :type "/Game/War3/GameBase/BP_War3GameMode Object Reference"))
  (bind _asbp_war_3game_mode (cast `/Game/War3/GameBase/BP_War3GameMode` (`GameplayStatics.GetGameMode` null))
    (:`then`
      (return _asbp_war_3game_mode))
    (:`CastFailed`
      (`KismetSystemLibrary.PrintString` null "GameMode Can't Cast To BP_War3GameMode" true true (struct :`R` 1.0 :`A` 1.0) 10.0))))

(fn `FastGetWarPlayerController`
  (returns (`AsBP War 3Player Controller` :type "/Game/War3/GameBase/BP_War3PlayerController Object Reference"))
  (bind _asbp_war_3player_controller (cast `/Game/War3/GameBase/BP_War3PlayerController` (`GameplayStatics.GetPlayerController` null))
    (:`then`
      (return _asbp_war_3player_controller))
    (:`CastFailed`
      (`KismetSystemLibrary.PrintString` null "PlayerController Can't Cast To BP_War3PlayerController" true true (struct :`R` 1.0 :`A` 1.0) 10.0))))