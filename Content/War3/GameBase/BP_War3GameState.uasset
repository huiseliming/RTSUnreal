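; War3 game state Blueprint that drives the sun and sky from the game clock, giving a time-of-day cycle.
; On BeginPlay it caches the first DirectionalLight and the first BP_Sky_Sphere found in the level.
; Every Tick it sets the light's pitch from scaled game time, then tells the sky sphere to update its sun direction to match.
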(event `self.ReceiveBeginPlay`
  (`parent.ReceiveBeginPlay`)
  (`|ExecutionSequence`
    (:`then_0`
      (bind _outactors (`GameplayStatics.GetAllActorsOfClass` "/Script/Engine.DirectionalLight"))
      (set `self.SunLight` (`|GetArrayItem` _outactors)))
    (:`then_1`
      (bind _outactors_2 (`GameplayStatics.GetAllActorsOfClass` "/Engine/EngineSky/BP_Sky_Sphere.BP_Sky_Sphere_C"))
      (set `self.SkyShpere` (`|GetArrayItem` _outactors_2)))))

(event `self.ReceiveTick`
  (params (DeltaSeconds :type "Float (single-precision)"))
  (`parent.ReceiveTick` DeltaSeconds)
  (`self.K2_SetActorRotation` (`self.SunLight`) (`KismetMathLibrary.MakeRotator` 0.0 (/ (`self.GetGameTime`) 240.0)) false)
  (`/Engine/EngineSky/BP_Sky_Sphere.UpdateSunDirection` (`self.SkyShpere`)))

(fn `UserConstructionScript`)